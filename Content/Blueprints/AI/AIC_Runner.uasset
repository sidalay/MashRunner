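; AIC_Runner is an AI controller that drives a possessed BP_Runner by faking alternating left and right power inputs.
; On possess it caches the runner, and on BeginPlay it starts a one-shot timer with a random delay between configurable minimum and maximum values.
; A FlipFlop in the simulated input event alternates the runner's left and right power calls, re-arming the randomized timer after each.
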(event Custom|SimualteInput
  (bind _owningrunner (Variables|Default|GetOwningRunner))
  (Utilities|FlowControl|FlipFlop
    (:A
      (Default|SimulatePowerLeft _owningrunner)
      (CallFunction|SetInputDelay))
    (:B
      (Default|SimulatePowerRight _owningrunner)
      (CallFunction|SetInputDelay))))

(event EventBeginPlay
  (CallFunction|SetInputDelay))

(event EventTick
  (params (DeltaSeconds :type Float%20%28single-precision%29)))

(event EventPossess
  (params (PossessedPawn :type Pawn%20Object%20Reference))
  (bind _asbp_runner (Utilities|Casting|CastToBP_Runner PossessedPawn))
  (Variables|Default|SetOwningRunner _asbp_runner))

(fn ConstructionScript)

(fn SetInputDelay
  (Utilities|Time|SetTimerbyEvent (EventDispatchers|CreateEvent :!event Custom|SimualteInput) (Math|Random|RandomFloatinRange (Variables|Default|GetMinInputDelay) (Variables|Default|GetMaxInputDelay))))